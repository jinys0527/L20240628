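; Base actor for one step of the VR content sequence, meant as a parent for concrete step actors.
; On BeginPlay it binds to the content-step change dispatcher on BP_VRGameState.
; EventChangeContentStep calls EventStartStep, an empty hook here, when the incoming step matches CurStep.
; EventEndStep asks the game state to switch to NextStep, so steps chain through the game state without referencing each other.
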(event EventBeginPlay
  (CallFunction|BIndContentStep) ; 이벤트 디스패처를 Bind
)

(event Collision|EventActorBeginOverlap
  (params (OtherActor :type Actor%20Object%20Reference)))

(event EventTick
  (params (DeltaSeconds :type Float%20%28single-precision%29)))

(fn ConstructionScript)

(fn BIndContentStep
  (bind _asbp_vrgame_state (Utilities|Casting|CastToBP_VRGameState (Game|GetGameState)))
  (EventDispatchers|BindEventtoEventDispatcherChangeContentStep _asbp_vrgame_state (EventDispatchers|CreateEvent :!event EventChangeContentStep)) ; 생성한 이벤트 디스패처의 특정 조건을 충족되면 이벤트를 수신하여\n아래에서 생성한 함수가 실행된다.\n\nContent Step이 해당될 경우 StartStep을 진행한다.
)

(fn EventStartStep)

(fn EventEndStep
  (bind _asbp_vrgame_state (Utilities|Casting|CastToBP_VRGameState (Game|GetGameState)))
  (Default|ChangeContentStep _asbp_vrgame_state (Variables|Default|GetNextStep)))

(fn EventChangeContentStep
  (params (ContentStep :type EN_ContentStep%20Enum :default "NewEnumerator0"))
  (if (Utilities|Enum|Equal(Enum) ContentStep (Variables|Default|GetCurStep))
    (CallFunction|EventStartStep)))