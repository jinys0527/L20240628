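; Step actor that teleports the player to the PlayerStart matching PlayerStartTag during a VR step sequence.
; On step start it blocks step changes through BP_VRGameState's CanChange and fades the camera out.
; Timers then run DoTeleport, which moves and rotates the pawn and fades back in, and EventEndStep, which re-enables step changes and ends the step.
; The construction script displays Direction on a TextRender.
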(event EventBeginPlay
  (|CallParentFunction) ; This node is disabled and will not be called.\nDrag off pins to build functionality.
)

(event Collision|EventActorBeginOverlap
  (params (OtherActor :type Actor%20Object%20Reference))
  (|CallParentFunction OtherActor) ; This node is disabled and will not be called.\nDrag off pins to build functionality.
)

(event EventTick
  (params (DeltaSeconds :type Float%20%28single-precision%29))
  (|CallParentFunction DeltaSeconds) ; This node is disabled and will not be called.\nDrag off pins to build functionality.
)

(fn ConstructionScript
  (|CallParentFunction)
  (Rendering|Components|TextRender|SetText (Variables|Default|GetTextRender) (Variables|Default|GetDirection)))

(fn EventStartStep
  (|CallParentFunction)
  (bind _asbp_vrgame_state (Utilities|Casting|CastToBP_VRGameState (Game|GetGameState)))
  (Variables|/Game/StepContent/Gamemode/BP_VRGameState.BP_VRGameState_C|SetCanChange _asbp_vrgame_state false) ; Teleport Step이 시작되면 Step이 \n변경되지 않게 설정
  (CameraFades|StartCameraFade :self (Game|GetPlayerCameraManager 0) :ToAlpha 1.0) ; FadeOut
  (Utilities|Time|SetTimerbyFunctionName 0 "DoTeleport" 5.0))

(fn DoTeleport
  (bind _returnvalue (Game|GetGameMode))
  (bind _playerstarttag (Variables|Default|GetPlayerStartTag))
  (bind _returnvalue_2 (Class|GameModeBase|FindPlayerStart _returnvalue 0 _playerstarttag))
  ;[1 1 1] PlayerStartTag와 같은 Tag를 가지는 PlayerStart의 위치를 찾아 플레이어의 위치와 방향을 PlayerStart로 이동시키는 단계
  (Transformation|SetActorLocationAndRotation (Game|Player|GetPlayerPawn 0) (Transformation|GetActorLocation _returnvalue_2) (Transformation|GetActorRotation _returnvalue_2))
  (CameraFades|StartCameraFade :self (Game|GetPlayerCameraManager 0) :FromAlpha 1.0 :bHoldWhenFinished true) ; FadeIn
  (Utilities|Time|SetTimerbyFunctionName 0 "EventEndStep" 5.0))

(fn EventEndStep
  (bind _asbp_vrgame_state (Utilities|Casting|CastToBP_VRGameState (Game|GetGameState)))
  (Variables|/Game/StepContent/Gamemode/BP_VRGameState.BP_VRGameState_C|SetCanChange _asbp_vrgame_state true)
  (|CallParentFunction))