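; Step actor that shows a popup widget with a title and description while its step runs, with optional audio.
; BeginPlay hides and fills the widget; for the level popup variant, it prefixes both texts with a zero-padded "LevelNN" parsed from the VR pawn's selected floor name.
; Starting the step shows the popup, then ends it when the sound finishes or, without sound, on a fallback timer.
; ClearStep hides it, stops audio and cancels that timer.
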(event EventBeginPlay
  (|CallParentFunction)
  (Rendering|SetVisibility (Variables|Default|GetWidget) false false)
  (bind _aswb_popup_widget (Utilities|Casting|CastToWB_PopupWidget (UserInterface|GetUserWidgetObject (Variables|Default|GetWidget))))
  (CallFunction|SetTitleDesc _aswb_popup_widget)
  (Audio|Components|Audio|SetSound (Variables|Default|GetAudio) (Variables|Default|GetSound))
  (EventDispatchers|BindEventtoOnAudioFinished (Variables|Default|GetAudio) (EventDispatchers|CreateEvent :!event EventSoundFinish)) ; Audio가 종료되면 아래의 함수가 실행됨
)

(fn ConstructionScript
  (|CallParentFunction))

(fn EventStartStep
  (|CallParentFunction)
  (Rendering|SetVisibility (Variables|Default|GetWidget) true false)
  (Variables|Default|GetSound ; Sound 파일이 존재한다면\nValid 아니면 Not Valid
    (:then
      (Audio|Components|Audio|Play (Variables|Default|GetAudio) 0.0))
    (:else
      (Utilities|Time|SetTimerbyFunctionName 0 "EventEndStep" 5.0))))

(fn EventSoundFinish
  (CallFunction|EventEndStep))

(fn EventEndStep
  (|CallParentFunction)
  (Rendering|SetVisibility (Variables|Default|GetWidget) false false))

(fn SetTitleDesc
  (params (PopupWidget :type WB%20Popup%20Widget%20Object%20Reference))
  (if (Utilities|Enum|Equal(Enum) (Variables|Default|GetCurStep) "NewEnumerator5")
    ;[1 1 1] LevelPopup일 때
    (bind _asbp_vrstep_pawn (Utilities|Casting|CastToBP_VRStepPawn (Game|Player|GetPlayerPawn 0)))
    (bind _selectedactorname (Default|GetSelectedActorName _asbp_vrstep_pawn)) ; 선택된 층의 이름을 받아오는 함수
    (bind _result (CallFunction|SetLevelName (Utilities|String|GetSubstring _selectedactorname 0 (Utilities|String|FindSubstring _selectedactorname "F" false true)))) ; Level의 이름 형태로 만들어주는 함수
    (Default|SetPopupText PopupWidget (Utilities|String|Append _result (Variables|Default|GetTitle)) (Utilities|String|Append _result (Variables|Default|GetDescription)))
    (else
      ;[1 1 1] LevelPopup이 아닐 때
      (Default|SetPopupText PopupWidget (Variables|Default|GetTitle) (Variables|Default|GetDescription)))))

(fn SetLevelName
  (params (String :type String))
  ;[1 1 1] 한 자리 수인지 확인
  (if (== (Utilities|String|Len String) 1)
    (bind _output_get (LocalVariables|SetLevelName (Utilities|String|Append "Level" (Utilities|String|Append "0" String))))
    (return _output_get)
    (else
      (bind _output_get_2 (LocalVariables|SetLevelName (Utilities|String|Append "Level" String)))
      (return _output_get_2))))

(fn GetFloorNumber
  (params (SelectActorName :type String))
  (return (Utilities|String|GetSubstring SelectActorName 0 (Utilities|String|FindSubstring SelectActorName "F" false true))))

(fn ClearStep
  (|CallParentFunction)
  (Utilities|FlowControl|Sequence
    (:then_0
      (Rendering|SetVisibility (Variables|Default|GetWidget) false false)
      (Audio|Components|Audio|Stop (Variables|Default|GetAudio)))
    (:then_1
      (if (Class|KismetSystemLibrary|TimerExists 0 "EventEndStep") ; 소리와 보이지 않게만 하면 \nEventEndStep을 타이머로 불러오던 게 \n남아서 지우기 위해 Condition의 \n함수에 대한 Timer가 존재한다면 Clear
        (Utilities|Time|ClearTimerbyFunctionName 0 "EventEndStep")))))