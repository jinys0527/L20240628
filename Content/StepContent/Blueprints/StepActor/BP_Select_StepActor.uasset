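; BP_Select_StepActor is a step actor for a VR step sequence in which the player selects a floor.
; It starts with its decal hidden and box collision off; starting the step enables collision and floor updating on BP_VRStepPawn.
; OnBeginOverlap and OnEndOverlap show and hide the decal as hover feedback.
; OnSelected disables floor updating and collision, hides the decal and ends the step.
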(event EventBeginPlay
  (|CallParentFunction)
  ;[1 1 1] 층 선택하는 Step이 되기 전 Visible, Collision을 꺼줌
  (Rendering|SetVisibility (Variables|Default|GetDecal) false false)
  (Collision|SetCollisionEnabled (Variables|Default|GetBox) "NoCollision"))

(event Collision|EventActorBeginOverlap
  (params (OtherActor :type Actor%20Object%20Reference))
  (|CallParentFunction OtherActor) ; This node is disabled and will not be called.\nDrag off pins to build functionality.
)

(event EventTick
  (params (DeltaSeconds :type Float%20%28single-precision%29))
  (|CallParentFunction DeltaSeconds) ; This node is disabled and will not be called.\nDrag off pins to build functionality.
)

(fn ConstructionScript
  (|CallParentFunction))

(fn EventStartStep
  (|CallParentFunction)
  (bind _asbp_vrstep_pawn (Utilities|Casting|CastToBP_VRStepPawn (Game|Player|GetPlayerPawn 0)))
  (Default|SetUpdateableFloor _asbp_vrstep_pawn true) ; 층 선택이 가능하게 하는 함수
  (Collision|SetCollisionEnabled (Variables|Default|GetBox) "QueryAndPhysics") ; 층의 Collision을 다시 켜서 Overlap이 가능하도록 함
)

(fn OnBeginOverlap
  (Rendering|SetVisibility (Variables|Default|GetDecal) true false) ; Overlap된 것을 보여주기 위해 Visible을 켜줌
)

(fn OnEndOverlap
  (Rendering|SetVisibility (Variables|Default|GetDecal) false false) ; Overlap이 끝난 걸 보여주기 위해 Visible을 꺼줌
)

(fn OnSelected
  (bind _asbp_vrstep_pawn (Utilities|Casting|CastToBP_VRStepPawn (Game|Player|GetPlayerPawn 0)))
  (Default|SetUpdateableFloor _asbp_vrstep_pawn false)
  (Collision|SetCollisionEnabled (Variables|Default|GetBox) "NoCollision")
  (Rendering|SetVisibility (Variables|Default|GetDecal) false false)
  (CallFunction|EventEndStep))