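; BP_FadeOut_StepActor is a step actor that fades the player's screen out as a step in a sequence.
; When the step starts, it runs the parent logic and starts a five-second camera fade on the player camera manager.
; A timer by function name then calls EventEndStep as the fade completes to end the step.
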(event EventBeginPlay
  (|CallParentFunction))

(event Collision|EventActorBeginOverlap
  (params (OtherActor :type Actor%20Object%20Reference))
  (|CallParentFunction OtherActor) ; This node is disabled and will not be called.\nDrag off pins to build functionality.
)

(event EventTick
  (params (DeltaSeconds :type Float%20%28single-precision%29))
  (|CallParentFunction DeltaSeconds) ; This node is disabled and will not be called.\nDrag off pins to build functionality.
)

(fn ConstructionScript
  (|CallParentFunction))

(fn EventStartStep
  (|CallParentFunction)
  (CameraFades|StartCameraFade :self (Game|GetPlayerCameraManager 0) :ToAlpha 1.0 :Duration 5.0)
  (Utilities|Time|SetTimerbyFunctionName 0 "EventEndStep" 5.0))